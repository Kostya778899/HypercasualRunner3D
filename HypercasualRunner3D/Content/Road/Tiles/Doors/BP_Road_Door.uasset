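; BP_Road_Door is a road tile door with a portal glass mesh that takes a random color.
; BeginPlay creates a dynamic material instance for the glass, then disables its collision for both Positive and Negative types and picks MainColor from a five-color palette.
; Reset re-runs the collision and material setup on the existing instance, re-rolling the color without recreating the material.
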(event EventBeginPlay
  (bind _portalglass (Variables|Default|GetPortalGlass))
  (bind _returnvalue (Rendering|Material|CreateDynamicMaterialInstance (Variables|Default|GetPortalGlass) 0 "/Game/Road/Tiles/Doors/Materials/MI_Road_Door.MI_Road_Door" "None" :!class /Script/Engine.PrimitiveComponent))
  (Variables|Default|SetPortalGlassMaterial _returnvalue)
  (Utilities|FlowControl|Sequence
    (:then_0
      (switch Utilities|FlowControl|Switch|SwitchonERoad_Door_Types (Variables|Default|GetType)
        (:NewEnumerator0
          (Collision|SetCollisionEnabled _portalglass "NoCollision"))
        (:NewEnumerator1
          (Collision|SetCollisionEnabled _portalglass "NoCollision"))))
    (:then_1
      (Rendering|Material|SetVectorParameterValue (Variables|Default|GetPortalGlassMaterial) "MainColor" (.OutItem (Utilities|Array|Random (Utilities|Array|MakeArray "(R=1.000000,G=1.000000,B=1.000000,A=1.000000)" "(R=1.000000,G=0.923462,B=0.000000,A=1.000000)" "(R=0.164040,G=0.000000,B=1.000000,A=1.000000)" "(R=1.000000,G=0.000000,B=0.493205,A=1.000000)" "(R=1.000000,G=0.507329,B=0.000000,A=1.000000)"))) :!class /Script/Engine.MaterialInstanceDynamic))
    (:then_2
      (Audio|Parameter|SetFloatParameter (Variables|Default|GetPortalGlassMaterial) "0,2" 1e+02 :!class /Script/AudioExtensions.AudioParameterControllerInterface))))

(event EventReset
  (bind _portalglass (Variables|Default|GetPortalGlass))
  (bind _portalglassmaterial (Variables|Default|GetPortalGlassMaterial))
  (Utilities|FlowControl|Sequence
    (:then_0
      (switch Utilities|FlowControl|Switch|SwitchonERoad_Door_Types (Variables|Default|GetType)
        (:NewEnumerator0
          (Collision|SetCollisionEnabled _portalglass "NoCollision"))
        (:NewEnumerator1
          (Collision|SetCollisionEnabled _portalglass "NoCollision"))))
    (:then_1
      (Rendering|Material|SetVectorParameterValue _portalglassmaterial "MainColor" (.OutItem (Utilities|Array|Random (Utilities|Array|MakeArray "(R=1.000000,G=1.000000,B=1.000000,A=1.000000)" "(R=1.000000,G=0.923462,B=0.000000,A=1.000000)" "(R=0.164040,G=0.000000,B=1.000000,A=1.000000)" "(R=1.000000,G=0.000000,B=0.493205,A=1.000000)" "(R=1.000000,G=0.507329,B=0.000000,A=1.000000)"))) :!class /Script/Engine.MaterialInstanceDynamic))
    (:then_2
      (Audio|Parameter|SetFloatParameter _portalglassmaterial "0,2" 1e+02 :!class /Script/AudioExtensions.AudioParameterControllerInterface))))

(fn ConstructionScript)