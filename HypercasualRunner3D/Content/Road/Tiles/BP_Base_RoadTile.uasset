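; Base road tile Blueprint that tracks the additional objects placed on it as child actors and resets them with the tile.
; On BeginPlay it gathers the direct ChildActorComponent children of AdditionObjectsScene into the AdditionObjects array.
; Its Reset event calls ResetMessage on each stored child actor, leaving the reset behavior to each object.
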(event EventBeginPlay
  (for _array_element (Components|GetChildrenComponents (Variables|Default|GetAdditionObjectsScene) false)
    (bind _aschild_actor_component (Utilities|Casting|CastToChildActorComponent _array_element))
    (Utilities|Array|Add (Variables|Default|GetAdditionObjects) _aschild_actor_component)))

(event EventReset
  (for _array_element (Variables|Default|GetAdditionObjects)
    (Class|BPIResetable|Reset(Message) (Variables|/Script/Engine.ChildActorComponent|GetChildActor _array_element))))

(fn ConstructionScript)