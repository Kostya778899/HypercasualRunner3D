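; BP_RoadGenerator is an actor that builds a straight road of CurrentTile actors along world +X on BeginPlay.
; Each tile spawns one scaled grid step past the last one in the Tiles array, starting at the generator's location.
; MoveTiles recycles the first tile to the road's end, rotates the array and resets the new first tile.
; The half-second loop that calls MoveTiles is disconnected, so the road stays static.
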(event EventBeginPlay
  (Utilities|FlowControl|Sequence
    (:then_0
      (for _index (range 0 (- (Variables|Default|GetTilesCount) 1))
        (bind _returnvalue (Game|SpawnActorfromClass (Variables|Default|GetCurrentTile) (Math|Transform|MakeTransform (CallFunction|GetNewTileSpawnPosition (Utilities|Struct|MakeIntVector 1 0 0)) "0, 0, 0" "1.000000,1.000000,1.000000") "Undefined" 0 0))
        (Utilities|Array|Add (Variables|Default|GetTiles) _returnvalue)))))

(fn ConstructionScript)

(fn GetNewTileSpawnPosition
  (params (Direction :type Int%20Vector%20Structure))
  (bind _tiles (Variables|Default|GetTiles))
  (if (> (Utilities|Array|Length (Variables|Default|GetTiles)) 0)
    (return (+ (Transformation|GetWorldLocation (Variables|/Script/Engine.Actor|GetRootComponent (Utilities|Array|Get(acopy) _tiles (- (Utilities|Array|Length _tiles) 1)))) (* Direction (Variables|Default|GetGridSize) (Variables|Default|GetGridScale))))
    (else
      (return (Transformation|GetActorLocation)))))

(fn MoveTiles
  (params (Direction :type Int%20Vector%20Structure))
  (bind _tiles (Variables|Default|GetTiles))
  (bind _output (Utilities|Array|Get(acopy) _tiles))
  (Transformation|SetActorLocation (Utilities|Array|Get(acopy) (Variables|Default|GetTiles)) (CallFunction|GetNewTileSpawnPosition Direction) false false)
  (Utilities|Array|Add _tiles _output)
  (Utilities|Array|RemoveIndex (Variables|Default|GetTiles))
  (Default|Reset _output))