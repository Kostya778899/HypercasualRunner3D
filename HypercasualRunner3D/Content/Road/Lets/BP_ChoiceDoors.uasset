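; BP_ChoiceDoors is a road obstacle that groups two BP_Door child actors and randomly picks one to differ from the other.
; On BeginPlay it caches both doors, sets all to one type, gives a random one the other type, then resets each so it can respond to its type.
; Its Reset event repeats the roll on the cached doors, so the choice can be reshuffled.
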(event EventBeginPlay
  (bind _doors (Variables|Default|GetDoors))
  (for _array_element (Utilities|Array|MakeArray (Variables|Default|GetBP_Door0) (Variables|Default|GetBP_Door1))
    (bind _asbp_door (Utilities|Casting|CastToBP_Door (Variables|/Script/Engine.ChildActorComponent|GetChildActor _array_element)))
    (Utilities|Array|Add (Variables|Default|GetDoors) _asbp_door))
  (Utilities|FlowControl|Sequence
    (:then_0
      (for _array_element_2 (Variables|Default|GetDoors)
        (Variables|/Game/Road/Lets/BP_Door.BP_Door_C|SetType _array_element_2 "NewEnumerator1")))
    (:then_1
      (Variables|/Game/Road/Lets/BP_Door.BP_Door_C|SetType (Utilities|Array|Get(acopy) _doors (Math|Random|RandomInteger (Utilities|Array|Length _doors))) "NewEnumerator0"))
    (:then_2
      (for _array_element_3 (Variables|Default|GetDoors)
        (Default|Reset _array_element_3)))))

(event EventReset
  (bind _doors (Variables|Default|GetDoors))
  (Utilities|FlowControl|Sequence
    (:then_0
      (for _array_element (Variables|Default|GetDoors)
        (Variables|/Game/Road/Lets/BP_Door.BP_Door_C|SetType _array_element "NewEnumerator1")))
    (:then_1
      (Variables|/Game/Road/Lets/BP_Door.BP_Door_C|SetType (Utilities|Array|Get(acopy) _doors (Math|Random|RandomInteger (Utilities|Array|Length _doors))) "NewEnumerator0"))
    (:then_2
      (for _array_element_2 (Variables|Default|GetDoors)
        (Default|Reset _array_element_2)))))

(fn ConstructionScript)