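; Road generator actor that spawns a straight row of tile actors along +X from its own location on BeginPlay.
; Each new tile is placed one scaled grid step beyond the last one in the Tiles array.
; MoveTiles recycles the oldest tile by moving it past the newest along a given direction, resetting it and shifting it to the array's end.
; A looping timer draws each tile's name and index as debug text.
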(event Custom|DrawDebugInterface
  (for (_array_element _array_index) (Variables|Default|GetTiles)
    (Rendering|Debug|DrawDebugString (+ (Transformation|GetActorLocation _array_element) "0,0,5.000000") (Utilities|String|Append (Utilities|GetObjectName _array_element) " (" (Utilities|String|ToString(Integer) _array_index) ")") 0 "(R=0.067708,G=0.031600,B=0.039067,A=1.000000)" 0.1)))

(event EventBeginPlay
  (Utilities|FlowControl|Sequence
    (:then_0
      (for _index (range 0 (- (Variables|Default|GetTilesCount) 1))
        (bind _returnvalue (Game|SpawnActorfromClass (Variables|Default|GetCurrentTile) (Math|Transform|MakeTransform (CallFunction|GetNewTileSpawnPosition (Utilities|Struct|MakeIntVector 1 0 0)) "0, 0, 0" "1.000000,1.000000,1.000000") "Undefined" 0 0))
        (Utilities|Array|Add (Variables|Default|GetTiles) _returnvalue))
      (Utilities|Time|SetTimerbyEvent (delegate Custom|DrawDebugInterface) 0.1 true))))

(fn ConstructionScript)

(fn GetNewTileSpawnPosition
  (params (Direction :type Int%20Vector%20Structure))
  (bind _tiles (Variables|Default|GetTiles))
  (if (> (Utilities|Array|Length (Variables|Default|GetTiles)) 0)
    (return (+ (Transformation|GetWorldLocation (Variables|/Script/Engine.Actor|GetRootComponent (Utilities|Array|Get(acopy) _tiles (- (Utilities|Array|Length _tiles) 1)))) (* Direction (Variables|Default|GetGridSize) (Variables|Default|GetGridScale))))
    (else
      (return (Transformation|GetActorLocation)))))

(fn MoveTiles
  (params (Direction :type Int%20Vector%20Structure))
  (bind _tiles (Variables|Default|GetTiles))
  (bind _output (Utilities|Array|Get(acopy) _tiles))
  (Transformation|SetActorLocation (Utilities|Array|Get(acopy) (Variables|Default|GetTiles)) (CallFunction|GetNewTileSpawnPosition Direction) false false)
  (Default|Reset _output)
  (Utilities|Array|Add _tiles _output)
  (Utilities|Array|RemoveIndex _tiles))